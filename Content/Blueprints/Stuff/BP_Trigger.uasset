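; BP_Trigger is a box trigger volume that relays overlap events to a set of actors in ActorToReact.
; When an actor of exactly the BP_Player class enters, it calls ReactMessage on each listed actor.
; On end overlap it calls EndReactMessage on each.
; The exit class check has no actor wired in and is negated, so it is not limited to the player.
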(event OnComponentBeginOverlap(Box)
  (params (OverlappedComponent :type Primitive%20Component%20Object%20Reference) (OtherActor :type Actor%20Object%20Reference) (OtherComp :type Primitive%20Component%20Object%20Reference) (OtherBodyIndex :type Integer) (bFromSweep :type Boolean) (SweepResult :type Hit%20Result%20Structure%20%28by%20ref%29))
  (if (== (Utilities|GetClass OtherActor) "/Game/Blueprints/BP_Player.BP_Player_C")
    (for _array_element (Variables|Default|GetActorToReact)
      (Class|BPIReact|React(Message) _array_element))))

(event OnComponentEndOverlap(Box)
  (params (OverlappedComponent :type Primitive%20Component%20Object%20Reference) (OtherActor :type Actor%20Object%20Reference) (OtherComp :type Primitive%20Component%20Object%20Reference) (OtherBodyIndex :type Integer))
  (if (not (== (Utilities|GetClass 0) "/Game/Blueprints/BP_Player.BP_Player_C"))
    (for _array_element (Variables|Default|GetActorToReact)
      (Class|BPIEndReact|EndReact(Message) _array_element))))

(fn ConstructionScript)