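; BP_Interactable is an interactable actor that registers with overlapping players and triggers reactions in other actors.
; Its Sphere's overlap events add or remove it from BPI_Player actors through UpdateInteractablesMessage.
; Interact sends ReactMessage to ActorsToReact, with optional once-only and destroy-on-interact checks, the latter only deregistering it from the sender.
; Snow-pile instances (Schnee) start with Sphere collision and overlaps off until EnableInteractable restores them.
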(event OnComponentBeginOverlap(Sphere)
  (params (OverlappedComponent :type Primitive%20Component%20Object%20Reference) (OtherActor :type Actor%20Object%20Reference) (OtherComp :type Primitive%20Component%20Object%20Reference) (OtherBodyIndex :type Integer) (bFromSweep :type Boolean) (SweepResult :type Hit%20Result%20Structure%20%28by%20ref%29))
  (if (Utilities|DoesObjectImplementInterface OtherActor "/Game/Blueprints/Interfaces/BPI_Player.BPI_Player_C")
    (Class|BPIPlayer|UpdateInteractables(Message) OtherActor self true)))

(event OnComponentEndOverlap(Sphere)
  (params (OverlappedComponent :type Primitive%20Component%20Object%20Reference) (OtherActor :type Actor%20Object%20Reference) (OtherComp :type Primitive%20Component%20Object%20Reference) (OtherBodyIndex :type Integer))
  (if (Utilities|DoesObjectImplementInterface OtherActor "/Game/Blueprints/Interfaces/BPI_Player.BPI_Player_C")
    (Class|BPIPlayer|UpdateInteractables(Message) OtherActor self false)))

(event Custom|EnableInteractable
  (Collision|SetCollisionEnabled (Variables|Default|GetSphere) "QueryAndPhysics")
  (Variables|/Script/Engine.PrimitiveComponent|SetbGenerateOverlapEvents (Variables|Default|GetSphere) true))

(event EventBeginPlay
  (if (Variables|Default|GetSchnee) ; checkt ob interactable schneehaufen is mit ja/nein
    (Collision|SetCollisionEnabled (Variables|Default|GetSphere) "NoCollision")
    (Variables|/Script/Engine.PrimitiveComponent|SetbGenerateOverlapEvents (Variables|Default|GetSphere) false)))

(event EventInteract
  (params (Sender :type Actor%20Object%20Reference))
  (Variables|Default|GetInteracctOnce
    (:then
      (Utilities|FlowControl|DoOnce false
        (:Completed
          _)))
    (:else
      _))
  (Class|BPIReact|React(Message) (Variables|Default|GetActorsToReact))
  (Variables|Default|GetDestroyOnInteract
    (:then
      (Class|BPIPlayer|UpdateInteractables(Message) Sender self false))
    (:else)))

(fn ConstructionScript)