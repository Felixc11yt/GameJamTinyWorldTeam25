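; Player controller Blueprint that sets up default input, camera pitch limits and pausing for the local player.
; On BeginPlay it adds the default Enhanced Input mapping context and clamps the camera manager's view pitch range.
; The pause input action pushes the pause widget onto the main UI stack, switches to UI-only input with the cursor shown, and pauses the game.
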(event Input|EnhancedActionEvents|EnhancedInputActionIA_Pause
  (params (ActionValue :type Boolean) (ElapsedSeconds :type Float%20%28double-precision%29) (TriggeredSeconds :type Float%20%28double-precision%29) (InputAction :type Input%20Action%20Object%20Reference :default "/Game/Inputs/IA_Pause.IA_Pause"))
  (:Started
    (bind _returnvalue (Class|CommonActivatableWidgetContainerBase|AddWidget (CallFunction|ReturnMainStack self) "/Game/Blueprints/UI/CAW_Pause.CAW_Pause_C"))
    (Input|SetInputModeUIOnly self _returnvalue "DoNotLock" true)
    (Variables|Default|SetbShowMouseCursor true)
    (Game|SetGamePaused true)))

(event EventBeginPlay
  (Input|AddMappingContext (PlayerController|LocalPlayerSubsystems|GetEnhancedInputLocalPlayerSubsystem) "/Game/Inputs/IMC_Default.IMC_Default" 0 "(bIgnoreAllPressedKeysUntilRelease=True,bForceImmediately=False,bNotifyUserSettings=False)")
  (Variables|/Script/Engine.PlayerCameraManager|SetViewPitchMax (Game|GetPlayerCameraManager 0) 5e+01)
  (Variables|/Script/Engine.PlayerCameraManager|SetViewPitchMin (Game|GetPlayerCameraManager 0) -8e+01))

(fn ConstructionScript)