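; BP_ICE is an ice surface volume that makes the player slide while standing inside it.
; When a BP_Player enters the Box, it lowers or replaces the character movement's ground friction and walking braking deceleration with configurable ice values.
; Leaving the Box restores both to hard-coded defaults rather than caching the player's previous values.
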(event OnComponentBeginOverlap(Box)
  (params (OverlappedComponent :type Primitive%20Component%20Object%20Reference) (OtherActor :type Actor%20Object%20Reference) (OtherComp :type Primitive%20Component%20Object%20Reference) (OtherBodyIndex :type Integer) (bFromSweep :type Boolean) (SweepResult :type Hit%20Result%20Structure%20%28by%20ref%29))
  (bind _asbp_player (Utilities|Casting|CastToBP_Player OtherActor))
  (Variables|/Script/Engine.CharacterMovementComponent|SetGroundFriction (Variables|/Script/Engine.Character|GetCharacterMovement _asbp_player) (Variables|Default|GetIce%20Ground%20Friction))
  (Variables|/Script/Engine.CharacterMovementComponent|SetBrakingDecelerationWalking (Variables|/Script/Engine.Character|GetCharacterMovement _asbp_player) (Variables|Default|GetIce%20Breaking%20Deceleration)))

(event OnComponentEndOverlap(Box)
  (params (OverlappedComponent :type Primitive%20Component%20Object%20Reference) (OtherActor :type Actor%20Object%20Reference) (OtherComp :type Primitive%20Component%20Object%20Reference) (OtherBodyIndex :type Integer))
  (bind _asbp_player (Utilities|Casting|CastToBP_Player OtherActor))
  (Variables|/Script/Engine.CharacterMovementComponent|SetGroundFriction (Variables|/Script/Engine.Character|GetCharacterMovement _asbp_player) 8.0)
  (Variables|/Script/Engine.CharacterMovementComponent|SetBrakingDecelerationWalking (Variables|/Script/Engine.Character|GetCharacterMovement _asbp_player) 2048.0))

(fn ConstructionScript)