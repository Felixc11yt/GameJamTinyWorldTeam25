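; BP_Collectable is a pickup that spins and bobs until the player collects it, adding its value to a tally via the game mode.
; A timeline started on BeginPlay animates the Scene component's rotation and height.
; The first BP_Player overlap with the Sphere starts a second timeline that lerps the actor toward a point below the player's origin.
; Once close enough, it sends Value to the game mode and destroys itself.
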(event OnComponentBeginOverlap(Sphere)
  (params (OverlappedComponent :type Primitive%20Component%20Object%20Reference) (OtherActor :type Actor%20Object%20Reference) (OtherComp :type Primitive%20Component%20Object%20Reference) (OtherBodyIndex :type Integer) (bFromSweep :type Boolean) (SweepResult :type Hit%20Result%20Structure%20%28by%20ref%29))
  (if (== (Utilities|GetClass OtherActor) "/Game/Blueprints/BP_Player.BP_Player_C")
    (Variables|Default|SetHItActor OtherActor)
    (Utilities|FlowControl|DoOnce false
      (:Completed
        (bind _value (Timeline|CollectTimeline Play)
          (:Update
            (bind _hitactor (Variables|Default|GetHItActor)
              (:then
                (Transformation|SetActorLocation (Math|Vector|Lerp(Vector) (Transformation|GetActorLocation) (- (Transformation|GetActorLocation _hitactor) "0.000000,0.000000,90.000000") _value) false false)
                (if (Utilities|Operators|EqualEqual (Transformation|GetActorLocation) (- (Transformation|GetActorLocation (Variables|Default|GetHItActor)) "0.000000,0.000000,90.000000") 2e+01)
                  (Class|BPIGameMode|IncreaseCollectableValue(Message) (Game|GetGameMode) (Variables|Default|GetValue))
                  (Actor|DestroyActor)))
              (:else))))))))

(event EventBeginPlay
  (bind (_direction _value _sine) (Timeline|Timeline Play)
    (:Update
      (Transformation|SetRelativeRotation (Variables|Default|GetScene) (Math|Rotator|Lerp(Rotator) "0, 0, 0" "0.000000,360.000000,0.000000" _value) false false)
      (Transformation|SetRelativeLocation (Variables|Default|GetScene) (Math|Vector|Lerp(Vector) "0.000000,0.000000,190.000000" "0.000000,0.000000,200.000000" _sine) true false))))

(fn ConstructionScript)