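; BP_Brief is a trigger that shows a letter-style brief widget to the player while they stand inside its sphere.
; On player overlap it waits briefly, creates the configurable BriefWidgetClass for player 0, adds it to the viewport and plays an open sound.
; On exit it plays a close sound and removes the widget after a one-second delay.
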(event OnComponentBeginOverlap(Sphere)
  (params (OverlappedComponent :type Primitive%20Component%20Object%20Reference) (OtherActor :type Actor%20Object%20Reference) (OtherComp :type Primitive%20Component%20Object%20Reference) (OtherBodyIndex :type Integer) (bFromSweep :type Boolean) (SweepResult :type Hit%20Result%20Structure%20%28by%20ref%29))
  (if (== (Utilities|GetClass OtherActor) "/Game/Blueprints/BP_Player.BP_Player_C")
    (Utilities|FlowControl|Delay 0.2)
    (bind _returnvalue (UserInterface|CreateWidget (Variables|Default|GetBriefWidgetClass) (Game|GetPlayerController 0)))
    (bind _output_get (Variables|Default|SetBriefWidget _returnvalue))
    (UserInterface|Viewport|AddtoViewport _output_get 0)
    (Audio|SpawnSound2D "/Game/Audio/UI/UI_LetterOpen.UI_LetterOpen" 1.0 1.0 0.0 0)))

(event OnComponentEndOverlap(Sphere)
  (params (OverlappedComponent :type Primitive%20Component%20Object%20Reference) (OtherActor :type Actor%20Object%20Reference) (OtherComp :type Primitive%20Component%20Object%20Reference) (OtherBodyIndex :type Integer))
  (if (== (Utilities|GetClass OtherActor) "/Game/Blueprints/BP_Player.BP_Player_C")
    (Audio|SpawnSound2D "/Game/Audio/UI/UI_LetterClose.UI_LetterClose" 1.0 1.0 0.0 0)
    (Utilities|FlowControl|Delay 1.0)
    (Widget|RemovefromParent (Variables|Default|GetBriefWidget))))

(fn ConstructionScript)