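; BP_Schnee is a snow interactable that restores the player's scale and camera position.
; Its static mesh starts hidden without collision until EnableSnow makes it visible and collidable.
; React plays a snow growth sound, waits briefly, then sets BP_Player's actor scale to normal and moves its camera to a fixed relative offset.
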(event Custom|EnableSnow
  (Rendering|SetVisibility (Variables|Default|GetStaticMesh) true false)
  (Collision|SetCollisionEnabled (Variables|Default|GetStaticMesh) "QueryAndPhysics"))

(event EventBeginPlay
  (Rendering|SetVisibility (Variables|Default|GetStaticMesh) false false)
  (Collision|SetCollisionEnabled (Variables|Default|GetStaticMesh) "NoCollision"))

(event EventReact
  (Audio|PlaySound2D "/Game/Audio/SFX_MainCharacter_Schneewachstum.SFX_MainCharacter_Schneewachstum" 1.0 1.0 0.0 0 0)
  (Utilities|FlowControl|Delay 1.3)
  (bind _asbp_player (Utilities|Casting|CastToBP_Player (Game|GetPlayerCharacter 0)))
  (Transformation|SetActorScale3D _asbp_player "1.000000,1.000000,1.000000")
  (Transformation|SetRelativeLocation (Variables|/Game/Blueprints/BP_Player.BP_Player_C|GetCamera _asbp_player) "-120.000000,0.000000,0.000000" false false))

(fn ConstructionScript)