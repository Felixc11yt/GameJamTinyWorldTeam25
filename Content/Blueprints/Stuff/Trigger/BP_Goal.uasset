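; Goal trigger that ends the game with an end screen once everything is collected (AlleGesammelt).
; Its React event checks that flag and runs a single time through a DoOnce.
; It switches to UI-only input, shows the cursor through BP_PlayerController and pauses the game, then adds the CAW_Ende widget after a zero-length Delay.
; The input mode's focus target, EndWidget, is only created afterwards.
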(event EventReact
  (bind _returnvalue (Game|GetPlayerController 0))
  (if (Variables|Default|GetAlleGesammelt)
    (Utilities|FlowControl|DoOnce false
      (:Completed
        (Input|SetInputModeUIOnly _returnvalue (Variables|Default|GetEndWidget) "DoNotLock" true)
        (bind _asbp_player_controller (Utilities|Casting|CastToBP_PlayerController _returnvalue))
        (Default|MouseCursorAn _asbp_player_controller)
        (Game|SetGamePaused true)
        (Utilities|FlowControl|Delay 0.0)
        (bind _returnvalue_2 (UserInterface|CreateWidget "/Game/Blueprints/UI/CAW_Ende.CAW_Ende_C" (Game|GetPlayerController 0)))
        (bind _output_get (Variables|Default|SetEndWidget _returnvalue_2))
        (UserInterface|Viewport|AddtoViewport _output_get 0)))))

(fn ConstructionScript)